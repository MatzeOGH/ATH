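; BP_test is a test pawn that probes the slope of the ground beneath it while driven by player input.
; MoveForward moves it along the control yaw, and LookRight turns the controller yaw.
; Each tick, a downward Visibility trace prints the dot products of the hit normal with the actor's forward and right vectors.
; Angle conversions of those dot products are present but unused.
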(event `self.ReceiveTick`
  (params (DeltaSeconds :type "Float (single-precision)"))
  (bind _returnvalue (`self.K2_GetActorLocation`))
  (bind (_outhit _returnvalue_2) (`KismetSystemLibrary.LineTraceSingle` _returnvalue (+ _returnvalue (0.0 0.0 -200.0)) "TraceTypeQuery1"))
  (if _returnvalue_2
    (bind (_bblockinghit _binitialoverlap _time _location _impactpoint _normal _impactnormal) (`GameplayStatics.BreakHitResult` _outhit))
    (`KismetSystemLibrary.PrintString` (`KismetStringLibrary.Concat_StrStr` "F: " (`KismetStringLibrary.Conv_DoubleToString` (`KismetMathLibrary.Dot_VectorVector` _impactnormal (`self.GetActorForwardVector`)))) true true (struct :`G` 0.66 :`B` 1.0 :`A` 1.0) 0.0)
    (`KismetSystemLibrary.PrintString` (`KismetStringLibrary.Concat_StrStr` "R: " (`KismetStringLibrary.Conv_DoubleToString` (`KismetMathLibrary.Dot_VectorVector` _impactnormal (`self.GetActorRightVector`)))) true true (struct :`G` 0.66 :`B` 1.0 :`A` 1.0) 0.0)))

(event `InputAxis|MoveForward`
  (params (AxisValue :type "Float (single-precision)"))
  (bind (_returnvalue_roll _returnvalue_pitch _returnvalue_yaw) (`KismetMathLibrary.BreakRotator` (`self.GetControlRotation`)))
  (`self.AddMovementInput` (`KismetMathLibrary.GetForwardVector` (`KismetMathLibrary.MakeRotator` 0.0 0.0 _returnvalue_yaw)) AxisValue))

(event `InputAxis|LookRight`
  (params (AxisValue :type "Float (single-precision)"))
  (`self.AddControllerYawInput` AxisValue))

(fn `UserConstructionScript`)