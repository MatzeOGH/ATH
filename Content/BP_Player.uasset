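; BP_Player is a motion-controller player that turns by holding one hand higher than the other.
; Each Tick maps the right-minus-left controller height difference to a clamped signed factor, scaled by MaxRotationPerSecond and delta time into a local yaw rotation.
; An angle-based approach remains unused: GetAngleBetweenVectors feeds only disconnected nodes, and the left/right helper GetMovementFromDegrees is never called.
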(event `self.ReceiveTick`
  (params (DeltaSeconds :type "Float (single-precision)"))
  (bind (_returnvalue_x _returnvalue_y _returnvalue_z) (`KismetMathLibrary.BreakVector` (`SceneComponent.K2_GetComponentLocation` (`self.MotionControllerLeft`))))
  (bind (_returnvalue_x_2 _returnvalue_y_2 _returnvalue_z_2) (`KismetMathLibrary.BreakVector` (`SceneComponent.K2_GetComponentLocation` (`self.MotionControllerRight`))))
  ;[1 1 1] Get difference between Z from Controllers and map them to range value for rotation
  (`self.K2_AddActorLocalRotation` (`KismetMathLibrary.MakeRotator` 0.0 0.0 (* DeltaSeconds (* (`KismetMathLibrary.MapRangeClamped` (- _returnvalue_z_2 _returnvalue_z) -10.0 10.0 -1.0 1.0) (`self.maxRotationPerSecond`))))))

(fn `GetAngleBetweenVectors`
  (params (InputA :type "Vector Structure") (InputB :type "Vector Structure"))
  (returns (DegreeBetweenVector :type "Float (double-precision)"))
  (return (`KismetMathLibrary.DegAcos` (`KismetMathLibrary.Dot_VectorVector` (`KismetMathLibrary.Normal` InputA) (`KismetMathLibrary.Normal` InputB)))))

(fn `GetMovementFromDegrees`
  (params (Degree :type "Float (double-precision)"))
  (returns (isLeft :type Boolean))
  ;[1 1 1] Check for degrees, if <0 it's left if > 0 it's right
  (if (< Degree 0.0)
    (if (> Degree -90.0)
      (set `self.isLeft` true)
      (else
        (set `self.isLeft` false :!label _label)))
    (else
      (goto _label)))
  (return (`self.isLeft`)))

(fn `UserConstructionScript`)